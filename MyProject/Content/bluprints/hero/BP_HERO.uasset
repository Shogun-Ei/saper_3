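; BP_HERO is the player hero character Blueprint, handling jump, dash and forward movement input.
; Jump press sets up a double jump with a short hold time before calling Jump, and release stops it.
; Dash works as a held sprint, raising max walk speed and a RunPR value until released.
; The forward axis moves the character along fixed world X rather than its facing direction.
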(event EventBeginPlay)

(event Collision|EventActorBeginOverlap
  (params (OtherActor :type Actor%20Object%20Reference)))

(event EventTick
  (params (DeltaSeconds :type Float%20%28single-precision%29)))

(event Input|ActionEvents|InputActiondash
  (params (Key :type Key%20Structure :default "None"))
  (:Pressed
    (Variables|Default|SetRunPR 1.5)
    (Variables|/Script/Engine.CharacterMovementComponent|SetMaxWalkSpeed (Variables|Character|GetCharacterMovement) 1e+03))
  (:Released
    (Variables|Default|SetRunPR 1.0)
    (Variables|/Script/Engine.CharacterMovementComponent|SetMaxWalkSpeed (Variables|Character|GetCharacterMovement) 6e+02)))

(event Input|ActionEvents|InputActionjump
  (params (Key :type Key%20Structure :default "None"))
  (:Pressed
    (Variables|Default|SetJumpMaxCount 2)
    (Variables|Default|SetJumpMaxHoldTime 0.3)
    (Character|Jump))
  (:Released
    (Character|StopJumping)))

(event Input|AxisEvents|InputAxisforvard
  (params (AxisValue :type Float%20%28single-precision%29))
  (Pawn|Input|AddMovementInput "1.000000,0.000000,0.000000" AxisValue false))

(fn ConstructionScript)